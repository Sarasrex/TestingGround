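; BPC_Scanner is a component that lets its owner trigger a scan.
; On BeginPlay it attaches itself to the player mesh fetched from the owner, keeping relative transforms.
; When the IA_Scan input completes, it spawns a BP_Scanner at the owner's location, passing in scan speed and maximum size.
; A CanScan flag and a delay enforce a cooldown between scans.
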(event `self.ReceiveBeginPlay`
  (bind _character_mesh (message `/Game/04BluePrints/Interfaces/BPI_Player.Get_Player_Mesh` (`self.GetOwner`)))
  (`self.K2_AttachToComponent` _character_mesh "None" "KeepRelative" "KeepRelative" "KeepRelative"))

(event `EnhancedInput|/Game/ThirdPerson/Input/Actions/IA_Scan`
  (params (ActionValue :type Boolean) (ElapsedSeconds :type "Float (double-precision)") (TriggeredSeconds :type "Float (double-precision)") (InputAction :type "InputAction Object Reference" :default "/Game/ThirdPerson/Input/Actions/IA_Scan.IA_Scan"))
  (:`Completed`
    (if (`self.Can_Scan?`)
      (set `self.Can_Scan?` false)
      (`|SpawnActorFromClass` "/Game/04BluePrints/BP_Scanner.BP_Scanner_C" (`KismetMathLibrary.MakeTransform` (`Actor.K2_GetActorLocation` (`self.GetOwner`))) "Undefined" "MultiplyWithRoot" null (`self.Scan_Speed`) (`self.Max_Scan_Size`) null)
      (`KismetSystemLibrary.Delay` (`self.Scan_CoolDown`))
      (set `self.Can_Scan?` true))))