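; BP_Scanner is an actor that acts as an expanding scan volume, growing until it reaches a size limit and then removing itself.
; Each Tick adds ScanSpeed scaled by delta time to its actor scale, keeping growth frame-rate independent.
; It destroys itself once the length of its scale vector reaches MaxScanSize, and the construction script is empty.
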(event `self.ReceiveTick`
  (params (DeltaSeconds :type "Float (single-precision)"))
  (`self.SetActorScale3D` (+ (`self.GetActorScale3D`) (* DeltaSeconds (`self.Scan_Speed`))))
  (if (>= (`KismetMathLibrary.VSize` (`self.GetActorScale3D`)) (`self.Max_Scan_Size`))
    (`self.K2_DestroyActor`)))

(fn `UserConstructionScript`)