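; Scanner pickup actor that animates its mesh, with the pickup itself unfinished.
; BeginPlay plays a timeline that lerps the mesh from its starting relative location toward its up vector scaled by a distance.
; Tick sets yaw from the mesh's Z location plus a speed-scaled delta, rather than accumulating rotation.
; The radius overlap checks for the player but does nothing, and an AddComponentMessage call is disconnected.
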(event `self.PickUp_Radius.OnComponentBeginOverlap`
  (params (OverlappedComponent :type "PrimitiveComponent Object Reference") (OtherActor :type "Actor Object Reference") (OtherComp :type "PrimitiveComponent Object Reference") (OtherBodyIndex :type Integer) (bFromSweep :type Boolean) (SweepResult :type "HitResult Structure (by ref)"))
  (if (== OtherActor (`GameplayStatics.GetPlayerCharacter` 0))
    _))

(event `self.ReceiveBeginPlay`
  ;[0 0.08896 1] Position
  (set `self.Scanner_Start_Position` (`SceneComponent.RelativeLocation` (`self.SM_Scanner`)))
  (`TimelineComponent.SetPlayRate` (`self.Scanner_PositionTimeline`) (/ 1.0 (`self.Position_Motion_In_Seconds`)))
  (bind (_direction _alpha) (`Timeline|Scanner_PositionTimeline`)
    (:`Update`
      (`SceneComponent.K2_SetRelativeLocation` (`self.SM_Scanner`) (`KismetMathLibrary.VLerp` (`self.Scanner_Start_Position`) (* (`KismetMathLibrary.GetUpVector` (`SceneComponent.RelativeRotation` (`self.SM_Scanner`))) (`self.UpDistance`)) _alpha) false false))))

(event `self.ReceiveTick`
  (params (DeltaSeconds :type "Float (single-precision)"))
  (bind (_relativelocation_x _relativelocation_y _relativelocation_z) (`KismetMathLibrary.BreakVector` (`SceneComponent.RelativeLocation` (`self.SM_Scanner`))))
  (`SceneComponent.K2_SetRelativeRotation` (`self.SM_Scanner`) (`KismetMathLibrary.MakeRotator` 0.0 0.0 (+ _relativelocation_z (* DeltaSeconds (`self.Rotation_Speed`)))) false false))

(fn `UserConstructionScript`)